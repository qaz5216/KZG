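; Interactable sliding attic middle door that the player opens and closes with the E key.
; Entering or leaving the box trigger enables or disables player input on the actor and toggles a prompt icon's visibility.
; E also toggles the icon, and a FlipFlop alternates eased MoveComponentTo calls that slide the door mesh sideways and back to its relative origin.
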(event `self.BoxColl.OnComponentBeginOverlap`
  (params (OverlappedComponent :type "PrimitiveComponent Object Reference") (OtherActor :type "Actor Object Reference") (OtherComp :type "PrimitiveComponent Object Reference") (OtherBodyIndex :type Integer) (bFromSweep :type Boolean) (SweepResult :type "HitResult Structure (by ref)"))
  (`self.EnableInput` (`GameplayStatics.GetPlayerController` 0))
  (`SceneComponent.ToggleVisibility` (`self.icon`) false :!label _label))

(event `self.BoxColl.OnComponentEndOverlap`
  (params (OverlappedComponent :type "PrimitiveComponent Object Reference") (OtherActor :type "Actor Object Reference") (OtherComp :type "PrimitiveComponent Object Reference") (OtherBodyIndex :type Integer))
  (`self.DisableInput` (`GameplayStatics.GetPlayerController` 0))
  (goto _label))

(event `Key|E`
  (params (Key :type "Key Structure"))
  (:`Pressed`
    (`SceneComponent.ToggleVisibility` (`self.icon`) false)))

(event `Key|E`
  (params (Key :type "Key Structure"))
  (bind _sm_doormidd (`self.SM_doormidd`))
  (:`Pressed`
    (`/Engine/EditorBlueprintResources/StandardMacros.FlipFlop`
      (:`A`
        (`|ExecutionSequence`
          (:`then_0`
            (`KismetSystemLibrary.MoveComponentTo` _sm_doormidd (0.0 -120.0 0.0) (struct) true true 2.0))))
      (:`B`
        (`|ExecutionSequence`
          (:`then_0`
            (`KismetSystemLibrary.MoveComponentTo` _sm_doormidd (0.0 0.0 0.0) (struct) true true 2.0)))))))

(fn `UserConstructionScript`)