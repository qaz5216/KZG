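; BP_Door3_2 is an interactive door that the player opens and closes with the Interact input, with a sound for each direction.
; A box trigger enables input and shows an icon while the player overlaps it, then disables both on exit.
; A timeline drives the door's relative yaw, and its current track value decides whether Interact plays it forward or reverses it.
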(event `self.BoxColl.OnComponentBeginOverlap`
  (params (OverlappedComponent :type "PrimitiveComponent Object Reference") (OtherActor :type "Actor Object Reference") (OtherComp :type "PrimitiveComponent Object Reference") (OtherBodyIndex :type Integer) (bFromSweep :type Boolean) (SweepResult :type "HitResult Structure (by ref)"))
  (if (== OtherActor (`GameplayStatics.GetPlayerCharacter` 0))
    (`self.EnableInput` (`GameplayStatics.GetPlayerController` 0))
    (`SceneComponent.SetVisibility` (`self.Icon`) true false)))

(event `self.BoxColl.OnComponentEndOverlap`
  (params (OverlappedComponent :type "PrimitiveComponent Object Reference") (OtherActor :type "Actor Object Reference") (OtherComp :type "PrimitiveComponent Object Reference") (OtherBodyIndex :type Integer))
  (if (== OtherActor (`GameplayStatics.GetPlayerCharacter` 0))
    (`self.DisableInput` (`GameplayStatics.GetPlayerController` 0))
    (`SceneComponent.SetVisibility` (`self.Icon`) false false)))

(event `InputAction|Interact`
  (params (Key :type "Key Structure"))
  (bind _returnvalue (`SceneComponent.K2_GetComponentLocation` (`self.DefaultSceneRoot`)))
  (:`Pressed`
    (if (< (stale _newtrack_0) 290.0)
      (`GameplayStatics.PlaySoundAtLocation` "/Game/Sound/SFX/DoorsAndFurnitures/SFX_DoorOpen_Cue.SFX_DoorOpen_Cue" _returnvalue (struct) 0.7 1.0 0.0 null null null null)
      (bind (_direction _newtrack_0) (`Timeline|Timeline_0` :!label _label)
        (:`Update`
          (`SceneComponent.K2_SetRelativeRotation` (`self.Door`) (`KismetMathLibrary.MakeRotator` 0.0 0.0 _newtrack_0) false false)))
      (else
        (`GameplayStatics.PlaySoundAtLocation` "/Game/Sound/SFX/DoorsAndFurnitures/SFX_DoorClose_Cue.SFX_DoorClose_Cue" _returnvalue (struct) 0.7 1.0 0.0 null null null null)
        (goto _label :!via `Reverse`)))))

(fn `UserConstructionScript`)