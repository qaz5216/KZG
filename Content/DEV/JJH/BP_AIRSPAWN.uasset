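; BP_AIRSPAWN is a spawner actor that triggers a one-time airplane drop event when the in-game time nears 8:00.
; Each Tick it looks up BP_Day and compares SolarTime within a small tolerance, gated by a DoOnce.
; The custom event then plays EndingDialogue_Cue at the actor's location and spawns BP_Airplane, passing it start and drop locations plus BP_DropProp.
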(event `self.ReceiveTick`
  (params (DeltaSeconds :type "Float (single-precision)"))
  (bind _returnvalue (`GameplayStatics.GetActorOfClass` "/Game/DEV/JJH/BP_Day.BP_Day_C"))
  (if (`KismetMathLibrary.NearlyEqual_FloatFloat` (`/Game/DEV/JJH/BP_Day.SolarTime` _returnvalue) 8.0 0.1)
    (`/Engine/EditorBlueprintResources/StandardMacros.DoOnce` false
      (:`Completed`
        (`self.CustomEvent`)))))

(event `CustomEvent`
  (`GameplayStatics.PlaySoundAtLocation` "/Game/CYS/DW_Ending/EndingDialogue_Cue.EndingDialogue_Cue" (`self.K2_GetActorLocation`) (struct) 1.0 1.0 0.0 null null null null)
  (bind _returnvalue (`|SpawnActorFromClass` "/Game/Airplane/BP_Airplane.BP_Airplane_C" (`self.Spawn Transform`) "Undefined" "MultiplyWithRoot" null null))
  (`AirPlane.MySetting` _returnvalue (`self.New Start Loc`) (`self.New Drop Loc`) "/Game/Airplane/BP_DropProp.BP_DropProp_C"))

(fn `airplane`)

(fn `UserConstructionScript`)