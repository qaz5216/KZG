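; Actor component for BP_ThirdPersonCharacter that handles building placement and toggles the WB_Build menu with its cursor, input mode and sounds.
; While Buildmode is on, Tick traces from the follow camera and moves a green, collision-free preview mesh to the hit point.
; A DoOnce limits preview setup to once per session.
; The Build input spawns the Building class at the preview transform, then clears the preview and exits build mode.
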(event `self.ReceiveBeginPlay`
  (bind _asbp_third_person_character (cast `/Game/HSH/Blueprints/BP_ThirdPersonCharacter` (`self.GetOwner`)))
  (set `self.As BP Third Person Character` _asbp_third_person_character)
  (set `self.Follow Camera` (`KZGCharacter.FollowCamera` _asbp_third_person_character)))

(event `self.ReceiveTick`
  (params (DeltaSeconds :type "Float (single-precision)"))
  (if (`self.buildmode`)
    (`self.loop`)))

(event `loop`
  (bind (_returnvalue_location _returnvalue_rotation) (`KismetMathLibrary.BreakTransform` (`SceneComponent.K2_GetComponentToWorld` (`self.Follow Camera`))))
  (bind (_outhit _returnvalue) (`KismetSystemLibrary.LineTraceSingle` _returnvalue_location (+ _returnvalue_location (* (`KismetMathLibrary.GetForwardVector` _returnvalue_rotation) 700.0)) "TraceTypeQuery1"))
  (if _returnvalue
    (`|ExecutionSequence`
      (:`then_0`
        (`/Engine/EditorBlueprintResources/StandardMacros.DoOnce` false :!label _label
          (:`Completed`
            (`/Engine/EditorBlueprintResources/StandardMacros.IsValid` (`self.Previewmesh`)
              (:`Is Valid`
                _)
              (:`Is Not Valid`
                (bind _returnvalue_2 (`|AddComponentByClass` (`self.As BP Third Person Character`) "/Script/Engine.StaticMeshComponent" false (`self.build preview transform`)))))
            (bind _output_get (set `self.Previewmesh` _returnvalue_2))
            (`StaticMeshComponent.SetStaticMesh` _output_get (`self.Previewstaticmesh`))
            (bind _returnvalue_3 (`MeshComponent.GetMaterialIndex` _output_get "None"))
            (for (_ _array_index) (`|MakeArray` _returnvalue_3 _returnvalue_3 _returnvalue_3 _returnvalue_3 _returnvalue_3 _returnvalue_3 _returnvalue_3 _returnvalue_3 _returnvalue_3 _returnvalue_3 _returnvalue_3 _returnvalue_3 _returnvalue_3 _returnvalue_3 _returnvalue_3 _returnvalue_3 _returnvalue_3 _returnvalue_3 _returnvalue_3 _returnvalue_3)
              (`PrimitiveComponent.SetMaterial` _output_get _array_index "/Game/DEV/JJH/M_green.M_green")
              (`PrimitiveComponent.SetCollisionEnabled` (`self.Previewmesh`) "NoCollision")))))
      (:`then_1`
        (bind _output_get_2 (set `self.build preview transform` (`KismetMathLibrary.MakeTransform` (`.Location` (`GameplayStatics.BreakHitResult` _outhit)))))
        (`SceneComponent.K2_SetWorldTransform` (`self.Previewmesh`) _output_get_2 false false)))))

(event `reset build`
  (goto _label :!via `Reset`))

(event `buildpreview`
  (bind _returnvalue (`GameplayStatics.GetPlayerController` 0))
  (if (not (`self.buildmode`))
    (set `PlayerController.bShowMouseCursor` true (`GameplayStatics.GetPlayerController` 0))
    (bind _returnvalue_2 (`|CreateWidget` "/Game/DEV/JJH/WB_Build.WB_Build_C"))
    (`UserWidget.AddToViewport` _returnvalue_2 0)
    (`WidgetBlueprintLibrary.SetInputMode_UIOnlyEx` (`GameplayStatics.GetPlayerController` 0) _returnvalue_2)
    (`GameplayStatics.PlaySound2D` "/Game/Sound/SFX/Footsteps/SFX_Inventory_Cue.SFX_Inventory_Cue" 1.0 1.0 0.0 null null)
    (else
      (`/Engine/EditorBlueprintResources/StandardMacros.IsValid` _returnvalue_2
        (:`Is Valid`
          (set `PlayerController.bShowMouseCursor` false _returnvalue)
          (`Widget.RemoveFromParent` _returnvalue_2)
          (`WidgetBlueprintLibrary.SetInputMode_GameOnly` _returnvalue)
          (`GameplayStatics.PlaySound2D` "/Game/Sound/SFX/Paper/SFX_Closed_Cue.SFX_Closed_Cue" 1.0 1.0 0.0 null null))))))

(event `Stopbuildmode`
  (set `self.buildmode` false)
  (bind _previewmesh (`self.Previewmesh`)
    (:`then`
      _)
    (:`else`
      _))
  (`StaticMeshComponent.SetStaticMesh` _previewmesh null)
  (set `self.Previewmesh` null)
  (`self.reset build`))

(event `spawnBuilding`
  (`|SpawnActorFromClass` (`self.building`) (`self.build preview transform`) "Undefined" "MultiplyWithRoot" null null)
  (`self.Stopbuildmode`))

(event `InputAction|Build`
  (params (Key :type "Key Structure"))
  (:`Pressed`
    (if (`self.buildmode`)
      (`self.spawnBuilding`))))