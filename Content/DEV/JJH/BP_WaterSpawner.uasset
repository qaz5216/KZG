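; BP_WaterSpawner is an interactable water purifier that produces water over time and stores it in its inventory component.
; On BeginPlay it starts a looping one-minute timer that adds one water item to ACInventory, calling MCUpdate when the add succeeds.
; Interacting opens the water tank view on the player's HUD for that inventory, and Lookat supplies the Korean "open water purifier" prompt.
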(event `self.ReceiveBeginPlay`
  (`self.WaterSpawn`))

(event `WaterSpawn`
  (`KismetSystemLibrary.K2_SetTimer` null "spawnwater" 60.0 true))

(event `/Game/DEV/JJH/Inventory/Interact_interface.InteractWith`
  (params (PlayerCharacter :type "/Game/HSH/Blueprints/BP_ThirdPersonCharacter Object Reference"))
  (`/Game/DEV/JJH/WB_PlayerHUD.showWaterTank` (`/Game/HSH/Blueprints/BP_ThirdPersonCharacter.HUD` PlayerCharacter) (`self.AC_Inventory`)))

(fn `Lookat`
  (returns (Message :type Text))
  (return (`|FormatText` "정수기 열기")))

(fn `spawnwater`
  (bind _ac_inventory (`self.AC_Inventory`))
  (bind _success (`/Game/DEV/JJH/Inventory/AC_Inventory.AddToInventory` _ac_inventory "water" 1))
  (if _success
    (`/Game/DEV/JJH/Inventory/AC_Inventory.MC_Update` _ac_inventory)))

(fn `UserConstructionScript`
  (`parent.UserConstructionScript`))