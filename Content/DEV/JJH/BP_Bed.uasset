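; Placeable bed piece for the player's building system, with placement-preview feedback.
; Overlap events on component R set the building system's Isoverlap flag and swap the preview between M_green and M_green_2.
; The build event applies BasicShapeMaterial and switches collision to the Block profile.
; Interactwith and Lookat are empty stubs; logic to advance BP_Day to the next day is present but disconnected.
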(event `self.ReceiveBeginPlay`)

(event `build`
  (bind _returnvalue (`MeshComponent.GetMaterialIndex` (`self.r`) "None"))
  (cast `/Game/HSH/Blueprints/BP_ThirdPersonCharacter` (`GameplayStatics.GetPlayerCharacter` 0))
  (for (_ _array_index) (`|MakeArray` _returnvalue _returnvalue _returnvalue _returnvalue _returnvalue _returnvalue _returnvalue)
    (`PrimitiveComponent.SetMaterial` (`self.r`) _array_index "/Engine/BasicShapes/BasicShapeMaterial.BasicShapeMaterial")
    (`PrimitiveComponent.SetCollisionProfileName` (`self.r`) "Block" true)))

(event `self.r.OnComponentEndOverlap`
  (params (OverlappedComponent :type "PrimitiveComponent Object Reference") (OtherActor :type "Actor Object Reference") (OtherComp :type "PrimitiveComponent Object Reference") (OtherBodyIndex :type Integer))
  (bind _returnvalue (`MeshComponent.GetMaterialIndex` (`self.r`) "None"))
  (bind _asbp_third_person_character (cast `/Game/HSH/Blueprints/BP_ThirdPersonCharacter` (`GameplayStatics.GetPlayerCharacter` 0)))
  (set `/Game/DEV/JJH/ACBP_BuildingSystem.isoverlap` false (`/Game/HSH/Blueprints/BP_ThirdPersonCharacter.ACBP_BuildingSystem` _asbp_third_person_character))
  (for (_ _array_index) (`|MakeArray` _returnvalue _returnvalue _returnvalue _returnvalue _returnvalue _returnvalue _returnvalue)
    (`PrimitiveComponent.SetMaterial` (`self.r`) _array_index "/Game/DEV/JJH/M_green.M_green")))

(event `self.r.OnComponentBeginOverlap`
  (params (OverlappedComponent :type "PrimitiveComponent Object Reference") (OtherActor :type "Actor Object Reference") (OtherComp :type "PrimitiveComponent Object Reference") (OtherBodyIndex :type Integer) (bFromSweep :type Boolean) (SweepResult :type "HitResult Structure (by ref)"))
  (bind _returnvalue (`MeshComponent.GetMaterialIndex` (`self.r`) "None"))
  (bind _asbp_third_person_character (cast `/Game/HSH/Blueprints/BP_ThirdPersonCharacter` (`GameplayStatics.GetPlayerCharacter` 0)))
  (set `/Game/DEV/JJH/ACBP_BuildingSystem.isoverlap` true (`/Game/HSH/Blueprints/BP_ThirdPersonCharacter.ACBP_BuildingSystem` _asbp_third_person_character))
  (for (_ _array_index) (`|MakeArray` _returnvalue _returnvalue _returnvalue _returnvalue _returnvalue _returnvalue _returnvalue)
    (`PrimitiveComponent.SetMaterial` (`self.r`) _array_index "/Game/DEV/JJH/M_green_2.M_green_2")))

(event `/Game/DEV/JJH/Inventory/Interact_interface.InteractWith`
  (params (PlayerCharacter :type "/Game/HSH/Blueprints/BP_ThirdPersonCharacter Object Reference")))

(fn `Lookat`
  (returns (Message :type Text))
  (return ""))

(fn `UserConstructionScript`)