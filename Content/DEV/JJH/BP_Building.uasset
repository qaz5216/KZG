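; BP_Building is a buildable actor with a SpawnMesh, tied to the player's ACBPBuildingSystem component.
; Its build event casts the player to BP_ThirdPersonCharacter, then sets materials on a list of SpawnMesh slot indices.
; Overlap, move and setMesh events are empty.
; Disconnected logic would update the component's overlap flag, recolor the mesh if it is the spawned one, swap meshes and choose materials by selection flags, but never runs.
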(event `self.ReceiveBeginPlay`)

(event `setMesh`)

(event `build`
  (bind _returnvalue (`MeshComponent.GetMaterialIndex` (`self.SpawnMesh`) "None"))
  (cast `/Game/HSH/Blueprints/BP_ThirdPersonCharacter` (`GameplayStatics.GetPlayerCharacter` 0))
  (for (_ _array_index) (`|MakeArray` _returnvalue _returnvalue _returnvalue _returnvalue _returnvalue _returnvalue _returnvalue)
    (`PrimitiveComponent.SetMaterial` (`self.SpawnMesh`) _array_index null)))

(event `self.SpawnMesh.OnComponentEndOverlap`
  (params (OverlappedComponent :type "PrimitiveComponent Object Reference") (OtherActor :type "Actor Object Reference") (OtherComp :type "PrimitiveComponent Object Reference") (OtherBodyIndex :type Integer)))

(event `move`)

(event `self.SpawnMesh.OnComponentBeginOverlap`
  (params (OverlappedComponent :type "PrimitiveComponent Object Reference") (OtherActor :type "Actor Object Reference") (OtherComp :type "PrimitiveComponent Object Reference") (OtherBodyIndex :type Integer) (bFromSweep :type Boolean) (SweepResult :type "HitResult Structure (by ref)")))

(fn `UserConstructionScript`)