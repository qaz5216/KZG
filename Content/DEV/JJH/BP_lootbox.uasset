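; BP_lootbox is a loot container actor that removes itself once its inventory is emptied.
; It responds to its inventory component's update event and checks whether the quantity has dropped to zero or below.
; When it has, it casts player 0's character to BP_ThirdPersonCharacter, removes that character's HUD menu from its parent, then destroys the actor.
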(event `self.AC_Inventory.OnInventoryUpdate`
  (if (<= (`/Game/DEV/JJH/Inventory/AC_Inventory.getQuantitiy` (`self.AC_Inventory`)) 0)
    (bind _asbp_third_person_character (cast `/Game/HSH/Blueprints/BP_ThirdPersonCharacter` (`GameplayStatics.GetPlayerCharacter` 0)))
    (`Widget.RemoveFromParent` (`/Game/DEV/JJH/WB_PlayerHUD.Menu` (`/Game/HSH/Blueprints/BP_ThirdPersonCharacter.HUD` _asbp_third_person_character)))
    (`self.K2_DestroyActor`)))

(fn `UserConstructionScript`
  (`parent.UserConstructionScript`))