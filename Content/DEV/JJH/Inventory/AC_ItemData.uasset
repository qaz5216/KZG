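; AC_ItemData is an actor component that makes its owner a pickup item carrying an ItemID and quantity.
; On BeginPlay it sets the owning actor to replicate.
; Interacting adds the item's row name and quantity to the player's ACInventory, destroying the owner only if the add succeeds.
; Its Lookat function is a stub returning an empty string.
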(event `self.ReceiveBeginPlay`
  (`Actor.SetReplicates` (`self.GetOwner`) true))

(event `/Game/DEV/JJH/Inventory/Interact_interface.InteractWith`
  (params (PlayerCharacter :type "/Game/HSH/Blueprints/BP_ThirdPersonCharacter Object Reference"))
  (bind _ac_inventory (`/Game/HSH/Blueprints/BP_ThirdPersonCharacter.AC_Inventory` PlayerCharacter))
  (bind (_itemid_datatable _itemid_rowname) (break `DataTableRowHandle` (`self.ItemID`)))
  (`/Engine/EditorBlueprintResources/StandardMacros.IsValid` _ac_inventory
    (:`Is Valid`
      (bind _success (`/Game/DEV/JJH/Inventory/AC_Inventory.AddToInventory` _ac_inventory _itemid_rowname (`self.Quantitiy`)))
      (if _success
        (`Actor.K2_DestroyActor` (`self.GetOwner`))))))

(fn `Lookat`
  (returns (Message :type Text))
  (return ""))