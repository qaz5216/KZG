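; BP_Hungryup is an inventory item effect actor that restores the player's hunger by a fixed amount.
; On BeginPlay it calls its Hungerup event, which casts player 0's character to BP_ThirdPersonCharacter and adds to its CurHungerP, with no clamping here.
; The effect fires once per spawn, and the actor does not destroy itself afterward.
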(event `self.ReceiveBeginPlay`
  (`parent.ReceiveBeginPlay`)
  (`self.Hungerup`))

(event `Hungerup`
  (bind _asbp_third_person_character (cast `/Game/HSH/Blueprints/BP_ThirdPersonCharacter` (`GameplayStatics.GetPlayerCharacter` 0)))
  (set `KZGCharacter.curHungerP` (+ (`KZGCharacter.curHungerP` _asbp_third_person_character) 40) _asbp_third_person_character))

(fn `UserConstructionScript`
  (`parent.UserConstructionScript`))