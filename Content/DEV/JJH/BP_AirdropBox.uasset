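; BP_AirdropBox is an interactable airdrop supply box that players open to access the items inside.
; Its look-at text is a Korean prompt to open the box, and interacting passes its AC_Inventory component to the player HUD's airdrop display.
; When an inventory update leaves the quantity at zero or below, it removes the HUD menu of player 0's BP_ThirdPersonCharacter and destroys itself.
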(event `self.AC_Inventory.OnInventoryUpdate`
  (if (<= (`/Game/DEV/JJH/Inventory/AC_Inventory.getQuantitiy` (`self.AC_Inventory`)) 0)
    (bind _asbp_third_person_character (cast `/Game/HSH/Blueprints/BP_ThirdPersonCharacter` (`GameplayStatics.GetPlayerCharacter` 0)))
    (`Widget.RemoveFromParent` (`/Game/DEV/JJH/WB_PlayerHUD.Menu` (`/Game/HSH/Blueprints/BP_ThirdPersonCharacter.HUD` _asbp_third_person_character)))
    (`self.K2_DestroyActor`)))

(event `/Game/DEV/JJH/Inventory/Interact_interface.InteractWith`
  (params (PlayerCharacter :type "/Game/HSH/Blueprints/BP_ThirdPersonCharacter Object Reference"))
  (`/Game/DEV/JJH/WB_PlayerHUD.show airdrop` (`/Game/HSH/Blueprints/BP_ThirdPersonCharacter.HUD` PlayerCharacter) (`self.AC_Inventory`)))

(fn `Lookat`
  (returns (Message :type Text))
  (return "항공 보급상자 열기"))

(fn `UserConstructionScript`
  (`parent.UserConstructionScript`))