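; BP_Box is an interactable central workbench that opens its inventory component as a container on the player's HUD and shows a Korean "open" prompt when looked at.
; On BeginPlay in Level_AlphaART_1, it spawns a rainy-day radio at its own transform if none exists.
; Every Tick it looks up BP_Day and, on day 3, plays the ending dialogue at its location through a DoOnce.
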(event `self.ReceiveBeginPlay`
  (bind _returnvalue (`GameplayStatics.GetCurrentLevelName` true))
  (if (`KismetStringLibrary.EqualEqual_StrStr` _returnvalue "Level_AlphaART_1")
    (bind _returnvalue_2 (`GameplayStatics.GetActorOfClass` (`self.Radio_Rainnyday`)))
    (`/Engine/EditorBlueprintResources/StandardMacros.IsValid` _returnvalue_2
      (:`Is Not Valid`
        (bind _returnvalue_3 (`|SpawnActorFromClass` (`self.Radio_Rainnyday`) (`self.GetTransform`) "AlwaysSpawn" "MultiplyWithRoot" null null))
        (bind _asradio_rainnyday (cast `/Game/CYS/Radio_Rainnyday` _returnvalue_3))))))

(event `self.ReceiveTick`
  (params (DeltaSeconds :type "Float (single-precision)"))
  (`self.3day`))

(event `3day`
  (bind _returnvalue (`GameplayStatics.GetActorOfClass` "/Game/DEV/JJH/BP_Day.BP_Day_C"))
  (if (== (`/Game/DEV/JJH/BP_Day.Day` _returnvalue) 3)
    (set `/Game/DEV/JJH/BP_Day.Day` 3 _returnvalue)
    (`/Engine/EditorBlueprintResources/StandardMacros.DoOnce` false
      (:`Completed`
        (`GameplayStatics.PlaySoundAtLocation` "/Game/CYS/DW_Ending/EndingDialogue_Cue.EndingDialogue_Cue" (`self.K2_GetActorLocation`) (struct) 1.0 1.0 0.0 null null null null)))))

(event `/Game/DEV/JJH/Inventory/Interact_interface.InteractWith`
  (params (PlayerCharacter :type "/Game/HSH/Blueprints/BP_ThirdPersonCharacter Object Reference"))
  (`/Game/DEV/JJH/WB_PlayerHUD.ShowContainer` (`/Game/HSH/Blueprints/BP_ThirdPersonCharacter.HUD` PlayerCharacter) (`self.AC_Inventory`)))

(fn `Lookat`
  (returns (Message :type Text))
  (return (`|FormatText` "중앙 작업대 열기")))

(fn `UserConstructionScript`)