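; BP_Bed1 is an interactable bed that fast-forwards the day cycle by eight hours, with a Korean "sleep" look-at prompt.
; Interacting switches the view to a CameraActor, shortens BP_Day's TotalTime1 and stores the wrapped wake-up hour through a DoOnce.
; Tick polls SolarTime against that hour with a small tolerance, then restores day speed, returns the view to the player and resets the DoOnce.
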(event `self.ReceiveBeginPlay`)

(event `run`
  (bind _returnvalue (`GameplayStatics.GetActorOfClass` "/Game/DEV/JJH/BP_Day.BP_Day_C"))
  (if (`KismetMathLibrary.NearlyEqual_FloatFloat` (`/Game/DEV/JJH/BP_Day.SolarTime` _returnvalue) (`self.Return Value Hours`) 0.05)
    (set `/Game/DEV/JJH/BP_Day.TotalTime1` 30.0 _returnvalue)
    (set `/Game/DEV/JJH/BP_Day.refresh` true _returnvalue)
    (bind _asbp_third_person_character (cast `/Game/HSH/Blueprints/BP_ThirdPersonCharacter` (`GameplayStatics.GetPlayerCharacter` 0)))
    (`PlayerController.SetViewTargetWithBlend` (`GameplayStatics.GetPlayerController` 0) _asbp_third_person_character 0.0 "VTBlend_Linear" 0.0 false)
    (goto _label :!via `Reset`)))

(event `self.ReceiveTick`
  (params (DeltaSeconds :type "Float (single-precision)"))
  (`self.run`))

(event `sleep`
  (bind _returnvalue (`GameplayStatics.GetActorOfClass` "/Game/DEV/JJH/BP_Day.BP_Day_C"))
  (set `/Game/DEV/JJH/BP_Day.TotalTime1` 0.3 _returnvalue)
  (`/Engine/EditorBlueprintResources/StandardMacros.DoOnce` false :!label _label
    (:`Completed`
      (bind _output_get (set `self.Return Value Hours` (+ (`/Game/DEV/JJH/BP_Day.SolarTime` _returnvalue) 8.0)))
      (if (> _output_get 24.0)
        (set `self.Return Value Hours` (- (`self.Return Value Hours`) 24.0))))))

(event `/Game/DEV/JJH/Inventory/Interact_interface.InteractWith`
  (params (PlayerCharacter :type "/Game/HSH/Blueprints/BP_ThirdPersonCharacter Object Reference"))
  (bind _returnvalue (`GameplayStatics.GetActorOfClass` "/Script/Engine.CameraActor"))
  (`PlayerController.SetViewTargetWithBlend` (`GameplayStatics.GetPlayerController` 0) _returnvalue 0.0 "VTBlend_Linear" 0.0 false)
  (`self.sleep`))

(fn `Lookat`
  (returns (Message :type Text))
  (return (`|FormatText` "잠자기")))

(fn `UserConstructionScript`)