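; Interactable bed prop that lets the player sleep until morning and recover stamina.
; Interacting while the player's Maxsize is low restores stamina and Maxsize, and changes BP_Day's TotalTime1 to fast-forward the day cycle.
; Every tick it checks BP_Day's SolarTime and resets TotalTime1 near 8:00, whether or not the player slept.
; Its Lookat prompt returns empty text.
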(event `self.ReceiveBeginPlay`)

(event `wakeupTime`
  (bind _returnvalue (`GameplayStatics.GetActorOfClass` "/Game/DEV/JJH/BP_Day.BP_Day_C"))
  (if (`KismetMathLibrary.NearlyEqual_FloatFloat` (`/Game/DEV/JJH/BP_Day.SolarTime` _returnvalue) 7.95 0.05)
    (set `/Game/DEV/JJH/BP_Day.TotalTime1` 5.0 _returnvalue)))

(event `self.ReceiveTick`
  (params (DeltaSeconds :type "Float (single-precision)"))
  (`self.wakeupTime`))

(event `sleep`
  (bind _asbp_third_person_character (cast `/Game/HSH/Blueprints/BP_ThirdPersonCharacter` (`GameplayStatics.GetPlayerCharacter` 0)))
  (if (< (`KZGCharacter.maxsize` _asbp_third_person_character) 250)
    (bind _returnvalue (`GameplayStatics.GetActorOfClass` "/Game/DEV/JJH/BP_Day.BP_Day_C"))
    (set `/Game/DEV/JJH/BP_Day.TotalTime1` 0.08 _returnvalue)
    (set `KZGCharacter.currentStamina` 700 _asbp_third_person_character)
    (set `KZGCharacter.playerStamina` 700 _asbp_third_person_character)
    (set `KZGCharacter.maxsize` 500 _asbp_third_person_character)))

(event `/Game/DEV/JJH/Inventory/Interact_interface.InteractWith`
  (params (PlayerCharacter :type "/Game/HSH/Blueprints/BP_ThirdPersonCharacter Object Reference"))
  (`self.sleep`))

(fn `Lookat`
  (returns (Message :type Text))
  (return ""))

(fn `UserConstructionScript`)