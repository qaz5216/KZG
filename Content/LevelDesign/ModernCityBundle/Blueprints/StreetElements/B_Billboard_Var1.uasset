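; Street billboard actor for the Modern City bundle that displays one of nine billboard variants with a matching point light.
; The construction script applies light intensity and visibility, then picks a variant from BillboardType or at random when RandomSelection is set.
; Each variant offsets SMBillboard's material through OffsetX/OffsetY in a 3x3 atlas layout and tints the light.
; The event graph has no gameplay logic.
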(event `self.ReceiveBeginPlay`)

(fn `UserConstructionScript`
  (bind _sm_billboard (`self.SM_Billboard`))
  (bind _sm_billboard_2 (`self.SM_Billboard`))
  (bind _sm_billboard_3 (`self.SM_Billboard`))
  (bind _sm_billboard_4 (`self.SM_Billboard`))
  (bind _sm_billboard_5 (`self.SM_Billboard`))
  (bind _sm_billboard_6 (`self.SM_Billboard`))
  (bind _sm_billboard_7 (`self.SM_Billboard`))
  (bind _sm_billboard_8 (`self.SM_Billboard`))
  (bind _sm_billboard_9 (`self.SM_Billboard`))
  (bind _sm_billboard_10 (`self.SM_Billboard`))
  (bind _sm_billboard_11 (`self.SM_Billboard`))
  (bind _sm_billboard_12 (`self.SM_Billboard`))
  (bind _sm_billboard_13 (`self.SM_Billboard`))
  (bind _sm_billboard_14 (`self.SM_Billboard`))
  (bind _sm_billboard_15 (`self.SM_Billboard`))
  (bind _sm_billboard_16 (`self.SM_Billboard`))
  (bind _sm_billboard_17 (`self.SM_Billboard`))
  (bind _sm_billboard_18 (`self.SM_Billboard`))
  (`LightComponent.SetIntensity` (`self.PointLight`) (`self.Light Intensity`))
  (`SceneComponent.SetVisibility` (`self.PointLight`) (`self.Light ON`) false)
  (if (`self.Random Selection`)
    (switch `/Game/LevelDesign/ModernCityBundle/Blueprints/StreetElements/E_Billboards` (cast `/Game/LevelDesign/ModernCityBundle/Blueprints/StreetElements/E_Billboards` (`KismetMathLibrary.Conv_IntToByte` (`KismetMathLibrary.RandomInteger` (- (enumcount `/Game/LevelDesign/ModernCityBundle/Blueprints/StreetElements/E_Billboards`) 0))))
      (:`NewEnumerator0`
        (`MeshComponent.SetScalarParameterValueOnMaterials` _sm_billboard_9 "OffsetX" 0.0)
        (`MeshComponent.SetScalarParameterValueOnMaterials` _sm_billboard_9 "OffsetY" 0.0)
        (`LightComponent.SetLightColor` (`self.PointLight`) (struct :`R` 0.072272 :`G` 0.3564 :`B` 0.47932 :`A` 1.0) true))
      (:`NewEnumerator1`
        (`MeshComponent.SetScalarParameterValueOnMaterials` _sm_billboard_13 "OffsetX" 0.33)
        (`MeshComponent.SetScalarParameterValueOnMaterials` _sm_billboard_13 "OffsetY" 0.0)
        (`LightComponent.SetLightColor` (`self.PointLight`) (struct :`R` 0.135633 :`G` 0.768151 :`B` 0.47932 :`A` 1.0) true))
      (:`NewEnumerator2`
        (`MeshComponent.SetScalarParameterValueOnMaterials` _sm_billboard_14 "OffsetX" 0.67)
        (`MeshComponent.SetScalarParameterValueOnMaterials` _sm_billboard_14 "OffsetY" 0.0)
        (`LightComponent.SetLightColor` (`self.PointLight`) (struct :`R` 1.0 :`G` 0.042311 :`B` 0.038204 :`A` 1.0) true))
      (:`NewEnumerator3`
        (`MeshComponent.SetScalarParameterValueOnMaterials` _sm_billboard_10 "OffsetX" 0.0)
        (`MeshComponent.SetScalarParameterValueOnMaterials` _sm_billboard_10 "OffsetY" 0.33)
        (`LightComponent.SetLightColor` (`self.PointLight`) (struct :`R` 0.026241 :`G` 0.296138 :`B` 0.665387 :`A` 1.0) true))
      (:`NewEnumerator4`
        (`MeshComponent.SetScalarParameterValueOnMaterials` _sm_billboard_11 "OffsetX" 0.33)
        (`MeshComponent.SetScalarParameterValueOnMaterials` _sm_billboard_11 "OffsetY" 0.33)
        (`LightComponent.SetLightColor` (`self.PointLight`) (struct :`R` 0.144128 :`G` 0.48515 :`B` 0.863157 :`A` 1.0) true))
      (:`NewEnumerator5`
        (`MeshComponent.SetScalarParameterValueOnMaterials` _sm_billboard_12 "OffsetX" 0.67)
        (`MeshComponent.SetScalarParameterValueOnMaterials` _sm_billboard_12 "OffsetY" 0.33)
        (`LightComponent.SetLightColor` (`self.PointLight`) (struct :`R` 0.520996 :`G` 0.14996 :`B` 1.0 :`A` 1.0) true))
      (:`NewEnumerator6`
        (`MeshComponent.SetScalarParameterValueOnMaterials` _sm_billboard_15 "OffsetX" 0.0)
        (`MeshComponent.SetScalarParameterValueOnMaterials` _sm_billboard_15 "OffsetY" 0.67)
        (`LightComponent.SetLightColor` (`self.PointLight`) (struct :`R` 0.973445 :`G` 0.351533 :`B` 0.036889 :`A` 1.0) true))
      (:`NewEnumerator7`
        (`MeshComponent.SetScalarParameterValueOnMaterials` _sm_billboard_16 "OffsetX" 0.33)
        (`MeshComponent.SetScalarParameterValueOnMaterials` _sm_billboard_16 "OffsetY" 0.67)
        (`LightComponent.SetLightColor` (`self.PointLight`) (struct :`R` 0.879622 :`G` 0.913099 :`B` 0.043735 :`A` 1.0) true))
      (:`NewEnumerator8`
        (`MeshComponent.SetScalarParameterValueOnMaterials` _sm_billboard_17 "OffsetX" 0.67)
        (`MeshComponent.SetScalarParameterValueOnMaterials` _sm_billboard_17 "OffsetY" 0.67)
        (`LightComponent.SetLightColor` (`self.PointLight`) (struct :`R` 0.879622 :`G` 0.381326 :`B` 0.022174 :`A` 1.0) true)))
    (else
      (switch `/Game/LevelDesign/ModernCityBundle/Blueprints/StreetElements/E_Billboards` (`self.BillboardType`)
        (:`NewEnumerator0`
          (`MeshComponent.SetScalarParameterValueOnMaterials` _sm_billboard_4 "OffsetX" 0.0)
          (`MeshComponent.SetScalarParameterValueOnMaterials` _sm_billboard_4 "OffsetY" 0.0)
          (`LightComponent.SetLightColor` (`self.PointLight`) (struct :`R` 0.072272 :`G` 0.3564 :`B` 0.47932 :`A` 1.0) true))
        (:`NewEnumerator1`
          (`MeshComponent.SetScalarParameterValueOnMaterials` _sm_billboard_5 "OffsetX" 0.33)
          (`MeshComponent.SetScalarParameterValueOnMaterials` _sm_billboard_5 "OffsetY" 0.0)
          (`LightComponent.SetLightColor` (`self.PointLight`) (struct :`R` 0.135633 :`G` 0.768151 :`B` 0.47932 :`A` 1.0) true))
        (:`NewEnumerator2`
          (`MeshComponent.SetScalarParameterValueOnMaterials` _sm_billboard_6 "OffsetX" 0.67)
          (`MeshComponent.SetScalarParameterValueOnMaterials` _sm_billboard_6 "OffsetY" 0.0)
          (`LightComponent.SetLightColor` (`self.PointLight`) (struct :`R` 1.0 :`G` 0.042311 :`B` 0.038204 :`A` 1.0) true))
        (:`NewEnumerator3`
          (`MeshComponent.SetScalarParameterValueOnMaterials` _sm_billboard "OffsetX" 0.0)
          (`MeshComponent.SetScalarParameterValueOnMaterials` _sm_billboard "OffsetY" 0.33)
          (`LightComponent.SetLightColor` (`self.PointLight`) (struct :`R` 0.026241 :`G` 0.296138 :`B` 0.665387 :`A` 1.0) true))
        (:`NewEnumerator4`
          (`MeshComponent.SetScalarParameterValueOnMaterials` _sm_billboard_18 "OffsetX" 0.33)
          (`MeshComponent.SetScalarParameterValueOnMaterials` _sm_billboard_18 "OffsetY" 0.33)
          (`LightComponent.SetLightColor` (`self.PointLight`) (struct :`R` 0.144128 :`G` 0.48515 :`B` 0.863157 :`A` 1.0) true))
        (:`NewEnumerator5`
          (`MeshComponent.SetScalarParameterValueOnMaterials` _sm_billboard_2 "OffsetX" 0.67)
          (`MeshComponent.SetScalarParameterValueOnMaterials` _sm_billboard_2 "OffsetY" 0.33)
          (`LightComponent.SetLightColor` (`self.PointLight`) (struct :`R` 0.520996 :`G` 0.14996 :`B` 1.0 :`A` 1.0) true))
        (:`NewEnumerator6`
          (`MeshComponent.SetScalarParameterValueOnMaterials` _sm_billboard_7 "OffsetX" 0.0)
          (`MeshComponent.SetScalarParameterValueOnMaterials` _sm_billboard_7 "OffsetY" 0.67)
          (`LightComponent.SetLightColor` (`self.PointLight`) (struct :`R` 0.973445 :`G` 0.313989 :`B` 0.036889 :`A` 1.0) true))
        (:`NewEnumerator7`
          (`MeshComponent.SetScalarParameterValueOnMaterials` _sm_billboard_8 "OffsetX" 0.33)
          (`MeshComponent.SetScalarParameterValueOnMaterials` _sm_billboard_8 "OffsetY" 0.67)
          (`LightComponent.SetLightColor` (`self.PointLight`) (struct :`R` 0.879622 :`G` 0.913099 :`B` 0.046665 :`A` 1.0) true))
        (:`NewEnumerator8`
          (`MeshComponent.SetScalarParameterValueOnMaterials` _sm_billboard_3 "OffsetX" 0.67)
          (`MeshComponent.SetScalarParameterValueOnMaterials` _sm_billboard_3 "OffsetY" 0.67)
          (`LightComponent.SetLightColor` (`self.PointLight`) (struct :`R` 0.896269 :`G` 0.514918 :`B` 0.022174 :`A` 1.0) true))))))