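; Interactive plastic balcony (variant 2) whose door slides when the player presses E near it.
; A trigger overlap enables input on the actor for the first player controller, and leaving disables it.
; E plays or reverses the Mover timeline based on IsOpen.
; The timeline's vector track sets the door's relative location, and each update derives IsOpen by comparing that vector to a fixed position.
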(event `self.Trigger.OnComponentBeginOverlap`
  (params (OverlappedComponent :type "PrimitiveComponent Object Reference") (OtherActor :type "Actor Object Reference") (OtherComp :type "PrimitiveComponent Object Reference") (OtherBodyIndex :type Integer) (bFromSweep :type Boolean) (SweepResult :type "HitResult Structure (by ref)"))
  (`self.EnableInput` (`GameplayStatics.GetPlayerController` 0)))

(event `Key|E`
  (params (Key :type "Key Structure"))
  (:`Pressed`
    (if (`self.IsOpen`)
      (bind (_direction _ismoving) (`Timeline|Mover` :!label _label)
        (:`Update`
          (set `self.IsOpen` (!= _ismoving (444.0 -137.0 120.0) :`ErrorTolerance` 0.0))
          (`SceneComponent.K2_SetRelativeLocation` (`self.Door`) _ismoving false false)))
      (else
        (goto _label :!via `Reverse`)))))

(event `self.Trigger.OnComponentEndOverlap`
  (params (OverlappedComponent :type "PrimitiveComponent Object Reference") (OtherActor :type "Actor Object Reference") (OtherComp :type "PrimitiveComponent Object Reference") (OtherBodyIndex :type Integer))
  (`self.DisableInput` (`GameplayStatics.GetPlayerController` 0)))

(fn `UserConstructionScript`)