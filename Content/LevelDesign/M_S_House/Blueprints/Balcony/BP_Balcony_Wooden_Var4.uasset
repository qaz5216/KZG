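; Wooden balcony Blueprint variant with four doors that open and close automatically through overlap triggers.
; Each trigger's begin overlap plays its own timeline, whose IsOpen track drives that door's relative yaw.
; End overlap reverses the timeline after a short delay, with no check on which actor overlapped or whether the trigger is still occupied.
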(event `self.Trigger1.OnComponentBeginOverlap`
  (params (OverlappedComponent :type "PrimitiveComponent Object Reference") (OtherActor :type "Actor Object Reference") (OtherComp :type "PrimitiveComponent Object Reference") (OtherBodyIndex :type Integer) (bFromSweep :type Boolean) (SweepResult :type "HitResult Structure (by ref)"))
  (bind (_direction _isopen) (`Timeline|Win1` :!label _label)
    (:`Update`
      (`SceneComponent.K2_SetRelativeRotation` (`self.Door1`) (`KismetMathLibrary.MakeRotator` 0.0 0.0 _isopen) false false))))

(event `self.Trigger1.OnComponentEndOverlap`
  (params (OverlappedComponent :type "PrimitiveComponent Object Reference") (OtherActor :type "Actor Object Reference") (OtherComp :type "PrimitiveComponent Object Reference") (OtherBodyIndex :type Integer))
  (`KismetSystemLibrary.Delay` 3.0)
  (goto _label :!via `Reverse`))

(event `self.Trigger2.OnComponentBeginOverlap`
  (params (OverlappedComponent :type "PrimitiveComponent Object Reference") (OtherActor :type "Actor Object Reference") (OtherComp :type "PrimitiveComponent Object Reference") (OtherBodyIndex :type Integer) (bFromSweep :type Boolean) (SweepResult :type "HitResult Structure (by ref)"))
  (bind (_direction _isopen) (`Timeline|Win2` :!label _label_2)
    (:`Update`
      (`SceneComponent.K2_SetRelativeRotation` (`self.Door2`) (`KismetMathLibrary.MakeRotator` 0.0 0.0 _isopen) false false))))

(event `self.Trigger2.OnComponentEndOverlap`
  (params (OverlappedComponent :type "PrimitiveComponent Object Reference") (OtherActor :type "Actor Object Reference") (OtherComp :type "PrimitiveComponent Object Reference") (OtherBodyIndex :type Integer))
  (`KismetSystemLibrary.Delay` 3.0)
  (goto _label_2 :!via `Reverse`))

(event `self.Trigger3.OnComponentBeginOverlap`
  (params (OverlappedComponent :type "PrimitiveComponent Object Reference") (OtherActor :type "Actor Object Reference") (OtherComp :type "PrimitiveComponent Object Reference") (OtherBodyIndex :type Integer) (bFromSweep :type Boolean) (SweepResult :type "HitResult Structure (by ref)"))
  (bind (_direction _isopen) (`Timeline|Win3` :!label _label_3)
    (:`Update`
      (`SceneComponent.K2_SetRelativeRotation` (`self.Door3`) (`KismetMathLibrary.MakeRotator` 0.0 0.0 _isopen) false false))))

(event `self.Trigger3.OnComponentEndOverlap`
  (params (OverlappedComponent :type "PrimitiveComponent Object Reference") (OtherActor :type "Actor Object Reference") (OtherComp :type "PrimitiveComponent Object Reference") (OtherBodyIndex :type Integer))
  (`KismetSystemLibrary.Delay` 3.0)
  (goto _label_3 :!via `Reverse`))

(event `self.Trigger4.OnComponentBeginOverlap`
  (params (OverlappedComponent :type "PrimitiveComponent Object Reference") (OtherActor :type "Actor Object Reference") (OtherComp :type "PrimitiveComponent Object Reference") (OtherBodyIndex :type Integer) (bFromSweep :type Boolean) (SweepResult :type "HitResult Structure (by ref)"))
  (bind (_direction _isopen) (`Timeline|Win4` :!label _label_4)
    (:`Update`
      (`SceneComponent.K2_SetRelativeRotation` (`self.Door4`) (`KismetMathLibrary.MakeRotator` 0.0 0.0 _isopen) false false))))

(event `self.Trigger4.OnComponentEndOverlap`
  (params (OverlappedComponent :type "PrimitiveComponent Object Reference") (OtherActor :type "Actor Object Reference") (OtherComp :type "PrimitiveComponent Object Reference") (OtherBodyIndex :type Integer))
  (`KismetSystemLibrary.Delay` 3.0)
  (goto _label_4 :!via `Reverse`))

(fn `UserConstructionScript`)