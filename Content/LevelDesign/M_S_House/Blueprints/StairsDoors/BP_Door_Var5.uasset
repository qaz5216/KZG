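; BP_Door_Var5 is an interactive door that the player toggles with the E key while inside its trigger.
; Trigger overlap enables or disables input and opens or closes a Gate that filters the key press.
; E sets IsPlayerUse on the door's AnimBP_Door according to IsOpen, then flips IsOpen after a delay.
; A failed anim instance cast draws a debug error string.
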(event `Key|E`
  (params (Key :type "Key Structure"))
  (:`Pressed`
    (`/Engine/EditorBlueprintResources/StandardMacros.Gate` true :!label _label
      (:`Exit`
        (if (`self.IsOpen`)
          (bind _asanim_bp_door (cast `/Game/LevelDesign/M_S_House/Meshes/Doors/AnimBP_Door` (`SkeletalMeshComponent.GetAnimInstance` (`self.Door`)))
            (:`then`
              (set `/Game/LevelDesign/M_S_House/Meshes/Doors/AnimBP_Door.IsPlayerUse` true _asanim_bp_door)
              (`KismetSystemLibrary.Delay` 2.0)
              (set `self.IsOpen` false))
            (:`CastFailed`
              (`KismetSystemLibrary.DrawDebugString` (0.0 0.0 0.0) "Error" null (struct :`R` 1.0 :`G` 1.0 :`B` 1.0 :`A` 1.0) 5.0 :!label _label_2)))
          (else
            (bind _asanim_bp_door_2 (cast `/Game/LevelDesign/M_S_House/Meshes/Doors/AnimBP_Door` (`SkeletalMeshComponent.GetAnimInstance` (`self.Door`)))
              (:`then`
                (set `/Game/LevelDesign/M_S_House/Meshes/Doors/AnimBP_Door.IsPlayerUse` false _asanim_bp_door_2)
                (`KismetSystemLibrary.Delay` 2.0)
                (set `self.IsOpen` true))
              (:`CastFailed`
                (goto _label_2)))))))))

(event `self.Trigger.OnComponentBeginOverlap`
  (params (OverlappedComponent :type "PrimitiveComponent Object Reference") (OtherActor :type "Actor Object Reference") (OtherComp :type "PrimitiveComponent Object Reference") (OtherBodyIndex :type Integer) (bFromSweep :type Boolean) (SweepResult :type "HitResult Structure (by ref)"))
  (`self.EnableInput` (`GameplayStatics.GetPlayerController` 0))
  (goto _label :!via `Open`))

(event `self.Trigger.OnComponentEndOverlap`
  (params (OverlappedComponent :type "PrimitiveComponent Object Reference") (OtherActor :type "Actor Object Reference") (OtherComp :type "PrimitiveComponent Object Reference") (OtherBodyIndex :type Integer))
  (`self.DisableInput` (`GameplayStatics.GetPlayerController` 0))
  (goto _label :!via `Close`))

(fn `UserConstructionScript`)