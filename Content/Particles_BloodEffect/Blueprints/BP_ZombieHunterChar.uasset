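; Zombie hunter character that can act as a posed performer in sword or pistol cinematics, chosen by an attack-type enum.
; The construction script sets up the weapon mesh, its transform and the animation data for that type.
; When cinematic, BeginPlay plays the single-node animation and disables input; the sword variant starts mid-slash, activates its camera and slows time via slomo.
; A helper function returns the player camera's location and rotation.
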(event `self.ReceiveBeginPlay`
  ;[0 0.2134 1] BEGIN PLAY
  ;[1 1 1] Check if cinematic is enabled
  (if (`self.IsCinematic?`)
    (`|ExecutionSequence`
      (:`then_0`
        ;[1 1 1] Update state accordingly
        (`self.Update State`))
      (:`then_1`
        ;[1 1 1] Disable input so the player cannot interfere with the animations
        (`self.DisableInput` (`GameplayStatics.GetPlayerController` 0))))))

(event `Update State`
  (bind _mesh (`self.Mesh`))
  (bind _mesh_2 (`self.Mesh`))
  ;[1 1 1] UPDATE STATE
  ;[1 1 1] Check if cinematic mode is enabled
  (if (`self.IsCinematic?`)
    (switch `/Game/Particles_BloodEffect/Blueprints/ENUM_AttackType` (`self.ENUM_AttackType`)
      (:`NewEnumerator0`
        ;[1 1 1] Sword Cinematic
        (`SkeletalMeshComponent.SetAnimationMode` _mesh_2 "AnimationSingleNode")
        (`SkeletalMeshComponent.SetAnimation` _mesh_2 "/Game/Particles_BloodEffect/Meshes/Mannequin/Animations/ANIM_Great_Sword_Slash.ANIM_Great_Sword_Slash")
        ;[1 1 1] Set Animation position
        (`SkeletalMeshComponent.SetPosition` _mesh_2 0.7 true)
        ;[1 1 1] Make sword camera active
        (`ActorComponent.SetActive` (`self.SwordCamera`) true false)
        ;[1 1 1] Play animation
        (`SkeletalMeshComponent.Play` (`self.Mesh`) false)
        ;[1 1 1] Slow down time
        (`KismetSystemLibrary.ExecuteConsoleCommand` "slomo 0.1" null))
      (:`NewEnumerator1`
        ;[1 1 1] Pistol Cinematic
        (`SkeletalMeshComponent.SetAnimationMode` _mesh "AnimationSingleNode")
        (`SkeletalMeshComponent.SetAnimation` _mesh "/Game/Particles_BloodEffect/Meshes/Mannequin/Animations/ANIM_Pistol_Idle.ANIM_Pistol_Idle")
        (`SkeletalMeshComponent.Play` _mesh true)))))

(fn `GetPlayerViewPoint`
  (returns (Location :type "Vector Structure") (Rotation :type "Rotator Structure"))
  (locals (MyPlayerController :type "PlayerController Object Reference"))
  (bind _playercameramanager (`PlayerController.PlayerCameraManager` (`local.MyPlayerController`)))
  (bind `_as플레이어_컨트롤러` (cast `PlayerController` (`self.GetController`)))
  (bind _output_get (set `local.MyPlayerController` `_as플레이어_컨트롤러`))
  (if (`KismetSystemLibrary.IsValid` _output_get)
    (if (`KismetSystemLibrary.IsValid` _playercameramanager)
      (return (`PlayerCameraManager.GetCameraLocation` _playercameramanager) (`PlayerCameraManager.GetCameraRotation` _playercameramanager)))))

(fn `UserConstructionScript`
  (bind _sword (`self.Sword`))
  (bind _sword_2 (`self.Sword`))
  (bind (_relativelocation_x _relativelocation_y _relativelocation_z) (`KismetMathLibrary.BreakVector` (`SceneComponent.RelativeLocation` _sword_2)))
  ;[1 1 1] Make these meshes visible
  (`SceneComponent.SetVisibility` (`self.Mesh`) true false)
  (`SceneComponent.SetVisibility` (`self.Sword`) true false)
  (if (`self.IsCinematic?`)
    (switch `/Game/Particles_BloodEffect/Blueprints/ENUM_AttackType` (`self.ENUM_AttackType`)
      (:`NewEnumerator0`
        ;[1 1 1] Setup for sword
        (`StaticMeshComponent.SetStaticMesh` _sword "/Game/Particles_BloodEffect/Meshes/Sword/SM_Sword.SM_Sword")
        (`SceneComponent.SetWorldScale3D` _sword (1.0 1.0 2.0))
        (set `SkeletalMeshComponent.AnimationData` (make `SingleAnimationPlayData` "/Game/Particles_BloodEffect/Meshes/Mannequin/Animations/ANIM_Great_Sword_Slash.ANIM_Great_Sword_Slash" false false) (`self.Mesh`)))
      (:`NewEnumerator1`
        ;[1 1 1] Setup for pistol
        (`StaticMeshComponent.SetStaticMesh` _sword_2 "/Game/Particles_BloodEffect/Meshes/Weapon/SM_Gun.SM_Gun")
        (`SceneComponent.K2_SetRelativeRotation` _sword_2 (`KismetMathLibrary.MakeRotator` 25.0 0.0 90.0) false false)
        (`SceneComponent.SetWorldScale3D` _sword_2 (0.2 0.2 0.2))
        (`SceneComponent.K2_SetRelativeLocation` _sword_2 (`KismetMathLibrary.MakeVector` (- _relativelocation_x 1.5) _relativelocation_y (- _relativelocation_z 7.0)) false false)
        (set `SkeletalMeshComponent.AnimationData` (make `SingleAnimationPlayData` "/Game/Particles_BloodEffect/Meshes/Mannequin/Animations/ANIM_Pistol_Idle.ANIM_Pistol_Idle" false false) (`self.Mesh`))))))