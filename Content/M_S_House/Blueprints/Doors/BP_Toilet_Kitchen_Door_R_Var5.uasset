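; Physics-driven interactive toilet/kitchen door that the player opens and closes with E while inside its trigger volume, which toggles input on overlap.
; When flagged closed, E shoves the simulated door with a fixed impulse; otherwise the Door_Driver timeline lerps it toward the frame's rotation.
; Each timeline update toggles physics off and on and sets IsClose, while any hit on the door clears that flag.
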(event `self.Door.OnComponentHit`
  (params (HitComponent :type "PrimitiveComponent Object Reference") (OtherActor :type "Actor Object Reference") (OtherComp :type "PrimitiveComponent Object Reference") (NormalImpulse :type "Vector Structure") (Hit :type "HitResult Structure (by ref)"))
  (set `self.IsClose?` false))

(event `Key|E`
  (params (Key :type "Key Structure"))
  (bind _door (`self.Door`))
  (:`Pressed`
    (if (`self.IsClose?`)
      (`PrimitiveComponent.AddImpulse` (`self.Door`) (-30000.0 -30000.0 0.0) "None" false)
      (set `self.IsClose?` false)
      (else
        (bind (_direction _mover) (`Timeline|Door_Driver` :!via `PlayFromStart`)
          (:`Update`
            (`SceneComponent.K2_SetRelativeRotation` _door (`KismetMathLibrary.RLerp` (`SceneComponent.K2_GetComponentRotation` _door) (`SceneComponent.K2_GetComponentRotation` (`self.Frame`)) _mover true) false false)
            (`PrimitiveComponent.SetSimulatePhysics` _door false)
            (`PrimitiveComponent.SetSimulatePhysics` _door true)
            (set `self.IsClose?` true)))))))

(event `self.Trigger.OnComponentBeginOverlap`
  (params (OverlappedComponent :type "PrimitiveComponent Object Reference") (OtherActor :type "Actor Object Reference") (OtherComp :type "PrimitiveComponent Object Reference") (OtherBodyIndex :type Integer) (bFromSweep :type Boolean) (SweepResult :type "HitResult Structure (by ref)"))
  (`self.EnableInput` (`GameplayStatics.GetPlayerController` 0)))

(event `self.Trigger.OnComponentEndOverlap`
  (params (OverlappedComponent :type "PrimitiveComponent Object Reference") (OtherActor :type "Actor Object Reference") (OtherComp :type "PrimitiveComponent Object Reference") (OtherBodyIndex :type Integer))
  (`self.DisableInput` (`GameplayStatics.GetPlayerController` 0)))

(fn `UserConstructionScript`)