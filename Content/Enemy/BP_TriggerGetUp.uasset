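; BP_TriggerGetUp is a trigger actor that rouses eating enemies when a KZGCharacter overlaps it.
; It scans all BP_Enemy actors and switches those whose FSM is in the Eating state to tracking that character.
; It then plays the discovery BGM cue and chains the chase-start cue when that finishes.
; Nothing disables the trigger, so each new overlap repeats the scan and music.
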(event `self.ReceiveActorBeginOverlap`
  (params (OtherActor :type "Actor Object Reference"))
  (bind _askzgcharacter (cast `KZGCharacter` OtherActor))
  (`|ExecutionSequence`
    (:`then_0`
      (bind _outactors (`GameplayStatics.GetAllActorsOfClass` "/Game/Enemy/BP_Enemy.BP_Enemy_C"))
      (for _array_element _outactors
        (bind _fsm (`Enemy.FSM` _array_element))
        (if (`|EnumEquality` (`EnemyFsm.mState` _fsm) "Eating")
          (`EnemyFsm.EatingToTrackingState` _fsm _askzgcharacter))))
    (:`then_1`
      (bind _returnvalue (`GameplayStatics.SpawnSound2D` "/Game/Sound/BGM/Trailer/BGM_Discover_Cue.BGM_Discover_Cue" 1.0 1.0 0.0 null))
      (add `AudioComponent.OnAudioFinished` _returnvalue (delegate `OnAudioFinished_이벤트`)))))

(event `OnAudioFinished_이벤트`
  (`GameplayStatics.PlaySound2D` "/Game/Sound/BGM/Dark_Music_Pack/WAV/BGM_ChaseStart_Cue.BGM_ChaseStart_Cue" 1.0 1.0 0.0 null null))

(fn `UserConstructionScript`)